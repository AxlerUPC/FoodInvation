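; Player character Blueprint with Enhanced Input movement and a switchable Idle, Melee or Rango (ranged) combat state.
; BeginPlay adds the player mapping context, movement input applies along world X and Y, and three state actions set and print the state.
; Attack input branches on state: Melee plays an override animation, guarded by an Attack flag until completed or cancelled.
; Rango calls Disparar, which spawns BP_Proyectil at the actor's transform.
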(event Input|EnhancedActionEvents|EnhancedInputActionIA_Attack
  (params (ActionValue :type Boolean) (ElapsedSeconds :type Float%20%28double-precision%29) (TriggeredSeconds :type Float%20%28double-precision%29) (InputAction :type Input%20Action%20Object%20Reference :default "/Game/GameContent/Input/Action/IA_Attack.IA_Attack"))
  (:Started
    (switch Utilities|FlowControl|Switch|SwitchonE_State (Variables|Default|GetState)
      (:NewEnumerator1
        (if (not (Variables|Character|GetAttack))
          (|PlayAnimationOverridewithCallbacks 0 0 "DefaultSlot" 1.0 0.0
            (:then
              (Variables|Character|SetAttack true))
            (:OnCompleted
              (Variables|Character|SetAttack false :!label _label))
            (:OnCancelled
              (goto _label)))))
      (:NewEnumerator2
        (CallFunction|Disparar)))))

(event Input|EnhancedActionEvents|EnhancedInputActionIA_StateIdle
  (params (ActionValue :type Boolean) (ElapsedSeconds :type Float%20%28double-precision%29) (TriggeredSeconds :type Float%20%28double-precision%29) (InputAction :type Input%20Action%20Object%20Reference :default "/Game/GameContent/Input/Action/IA_StateIdle.IA_StateIdle"))
  (:Started
    (Variables|Default|SetState "NewEnumerator0")
    (Development|PrintString "iDLE")))

(event Input|EnhancedActionEvents|EnhancedInputActionIA_Statemelee
  (params (ActionValue :type Boolean) (ElapsedSeconds :type Float%20%28double-precision%29) (TriggeredSeconds :type Float%20%28double-precision%29) (InputAction :type Input%20Action%20Object%20Reference :default "/Game/GameContent/Input/Action/IA_Statemelee.IA_Statemelee"))
  (:Started
    (Variables|Default|SetState "NewEnumerator1")
    (Development|PrintString "Melee" true true "(R=0.000000,G=1.000000,B=0.043210,A=1.000000)")))

(event Input|EnhancedActionEvents|EnhancedInputActionIA_StateRange
  (params (ActionValue :type Boolean) (ElapsedSeconds :type Float%20%28double-precision%29) (TriggeredSeconds :type Float%20%28double-precision%29) (InputAction :type Input%20Action%20Object%20Reference :default "/Game/GameContent/Input/Action/IA_StateRange.IA_StateRange"))
  (:Started
    (Variables|Default|SetState "NewEnumerator2")
    (Development|PrintString "Rango" true true "(R=1.000000,G=0.122771,B=0.182505,A=1.000000)")))

(event Input|EnhancedActionEvents|EnhancedInputActionIA_Movement
  (params (ActionValue :type Vector%202D%20Structure) (ElapsedSeconds :type Float%20%28double-precision%29) (TriggeredSeconds :type Float%20%28double-precision%29) (InputAction :type Input%20Action%20Object%20Reference :default "/Game/GameContent/Input/Action/IA_Movement.IA_Movement"))
  (Pawn|Input|AddMovementInput "1.000000,0.000000,0.000000" (.x ActionValue) false)
  (Pawn|Input|AddMovementInput "0.000000,1.000000,0.000000" (.y ActionValue) false))

(event EventBeginPlay
  (bind _asplayer_controller (Utilities|Casting|CastToPlayerController (Pawn|GetController)))
  (Input|AddMappingContext (PlayerController|LocalPlayerSubsystems|GetEnhancedInputLocalPlayerSubsystem _asplayer_controller) "/Game/GameContent/Input/IMC_Player.IMC_Player" 0 "(bIgnoreAllPressedKeysUntilRelease=True,bForceImmediately=False,bNotifyUserSettings=False)"))

(fn ConstructionScript
  (|CallParentFunction))

(fn Disparar
  (Game|SpawnActorfromClass "/Game/GameContent/Blueprint/Props/Proyectil/BP_Proyectil.BP_Proyectil_C" (Transformation|GetActorTransform) "Undefined" "MultiplyWithRoot" 0 0))