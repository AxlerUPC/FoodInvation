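; BPC_Health is a health component that tracks points and handles damage and healing.
; Damage and Heal both route through ChangeHealth, which clamps Points between zero and Limit and prints the new value.
; Event dispatchers broadcast Damaged and Healed after each change, while Death fires from ChangeHealth whenever the resulting points equal zero.
; GetPoints exposes the current value.
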(fn Damage
  (params (By :type Float%20%28double-precision%29))
  (bind _result (Math|Float|NegateFloat By)
    (:%20%20
      (CallFunction|ChangeHealth _result)
      (Default|CallDamaged))))

(fn ChangeHealth
  (params (By :type Float%20%28double-precision%29))
  (bind _output_get (Variables|Default|SetPoints (Math|Float|Clamp(Float) (+ (Variables|Default|GetPoints) By) 0.0 (Variables|Default|GetLimit))))
  (Development|PrintString (Utilities|String|ToString(Float) (Variables|Default|GetPoints)))
  (if (== _output_get 0.0)
    (Default|CallDeath)))

(fn Heal
  (params (By :type Float%20%28double-precision%29))
  (CallFunction|ChangeHealth By)
  (Default|CallHealed))

(fn GetPoints
  (return (Variables|Default|GetPoints)))