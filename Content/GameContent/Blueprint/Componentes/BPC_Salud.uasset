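; BPC_Salud is a health component that applies damage to its owner's life value.
; RecibirDaño subtracts the incoming damage from Vida and clamps it between zero and Vidamaxima.
; At zero it only prints a death message; otherwise it prints the remaining life and fires the SeRealizoDaño dispatcher.
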(fn RecibirDaño
  (params (Daño :type Float%20%28double-precision%29))
  (bind _output_get (Variables|Default|SetVida (Math|Float|Clamp(Float) (- (Variables|Default|GetVida) Daño) 0.0 (Variables|Default|GetVidamaxima))))
  (if (== _output_get 0.0)
    (Development|PrintString "Vida 0 Moriste")
    (Development|PrintString (Utilities|String|ToString(Float) _output_get))
    (else
      (Development|PrintString "Se quito vida" true true "(R=0.000000,G=0.660000,B=1.000000,A=1.000000)" 4.0)
      (Development|PrintString (Utilities|String|ToString(Float) _output_get) true true "(R=0.000000,G=0.660000,B=1.000000,A=1.000000)" 4.0)
      (Default|CallSeRealizoDaño))))