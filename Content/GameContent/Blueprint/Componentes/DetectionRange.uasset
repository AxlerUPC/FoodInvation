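; DetectionRange is a child actor that gives an enemy overlap-based detection of players, destroying itself if its parent lacks BPI_Enemy.
; When a BPI_Player actor begins overlapping, it sends that actor to the parent as attack target and cancels any pending timer.
; Any end overlap starts a TrackTime timer, if that value is non-negative, which clears the target on expiry.
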(event Custom|CustomEvent
  (Class|BPIEnemy|SetAttackTarget(Message) (Variables|Default|GetParent)))

(event EventBeginPlay
  (bind _returnvalue (Actor|GetParentActor))
  (if (Utilities|DoesObjectImplementInterface _returnvalue "/Game/GameContent/Blueprint/Interface/BPI_Enemy.BPI_Enemy_C")
    (Variables|Default|SetParent _returnvalue)
    (else
      (Actor|DestroyActor))))

(event Collision|EventActorBeginOverlap
  (params (OtherActor :type Actor%20Object%20Reference))
  (if (Utilities|DoesObjectImplementInterface OtherActor "/Game/GameContent/Blueprint/Interface/BPI_Player.BPI_Player_C")
    (Class|BPIEnemy|SetAttackTarget(Message) (Variables|Default|GetParent) OtherActor)
    (Utilities|Time|ClearandInvalidateTimerbyHandle (stale Collision|EventActorEndOverlap _returnvalue))))

(event Collision|EventActorEndOverlap
  (params (OtherActor :type Actor%20Object%20Reference))
  (bind _tracktime (Variables|Default|GetTrackTime))
  (if (>= _tracktime 0.0)
    (bind _returnvalue (Utilities|Time|SetTimerbyEvent (delegate Custom|CustomEvent) _tracktime))))

(fn ConstructionScript)