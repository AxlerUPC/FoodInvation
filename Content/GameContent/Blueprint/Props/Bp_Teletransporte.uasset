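; Teleporter prop that moves overlapping actors implementing BPI_Player to the location of a linked Destination.
; On overlap it checks that it is unoccupied and has a valid Destination, then calls Teleport on that Destination.
; Teleport marks the receiving pad Occupied before moving the passenger onto it, which prevents an immediate bounce back.
; The Occupied flag clears when any actor ends overlap with the pad.
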(event Collision|EventActorBeginOverlap
  (params (OtherActor :type Actor%20Object%20Reference))
  (bind _returnvalue (CallFunction|CanTeleport OtherActor))
  (if _returnvalue
    (CallFunction|Teleport (Variables|Default|GetDestination) OtherActor)))

(event Collision|EventActorEndOverlap
  (params (OtherActor :type Actor%20Object%20Reference))
  (Variables|Default|SetOccupied false))

(fn ConstructionScript)

(fn CanTeleport
  (params (TestObject :type Actor%20Object%20Reference))
  (return (Math|Boolean|ANDBoolean (Utilities|DoesObjectImplementInterface TestObject "/Game/GameContent/Blueprint/Interface/BPI_Player.BPI_Player_C") (not (Variables|Default|GetOccupied)) (Utilities|IsValid (Variables|Default|GetDestination)))))

(fn Teleport
  (params (Passenger :type Actor%20Object%20Reference))
  (if (not (Variables|Default|GetOccupied))
    (Variables|Default|SetOccupied true)
    (Transformation|SetActorLocation Passenger (Transformation|GetActorLocation self) false false)))