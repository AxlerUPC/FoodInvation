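; BP_Attack is an attack actor that damages overlapped actors implementing the BPI_Health interface.
; On overlap, ValidTarget checks for that interface, then DamageMessage passes Amount to the target.
; The attack destroys itself after a valid hit unless Piercing is set.
; A positive Duration also starts a timer on BeginPlay that destroys the actor when it expires.
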(event Custom|CustomEvent
  (Actor|DestroyActor))

(event EventBeginPlay
  (if (> (Variables|Default|GetDuration) 0.0)
    (Utilities|Time|SetTimerbyEvent (delegate Custom|CustomEvent) (Variables|Default|GetDuration))))

(event Collision|EventActorBeginOverlap
  (params (OtherActor :type Actor%20Object%20Reference))
  (bind _result (CallFunction|ValidTarget OtherActor))
  (if _result
    (Class|BPIHealth|Damage(Message) OtherActor (Variables|Default|GetAmount))
    (if (not (Variables|Default|GetPiercing))
      (Actor|DestroyActor))))

(fn ConstructionScript)

(fn ValidTarget
  (params (Actor :type Actor%20Object%20Reference))
  (return (Utilities|DoesObjectImplementInterface Actor "/Game/GameContent/Blueprint/Interface/BPI_Health.BPI_Health_C")))