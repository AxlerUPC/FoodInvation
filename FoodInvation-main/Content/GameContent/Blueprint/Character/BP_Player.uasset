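; BP_Player is the player character, switching between idle, melee and ranged states through Enhanced Input and attacking according to the current state.
; Melee spawns BP_PlayerMelee through BPCAttack and plays an animation override in the Attack slot, apparently using PaperZD.
; Ranged attacks play their animation and start a timed cooldown that resets gun charge.
; The ranged projectile spawn is unconnected, and charge decrements only when already negative.
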(event Custom|AttackAnim
  (params (AnimInstnace :type Paper%20ZD%20Anim%20Instance%20Object%20Reference) (AnimSequence :type Paper%20ZD%20Anim%20Sequence%20Object%20Reference))
  (|PlayAnimationOverridewithCallbacks AnimInstnace AnimSequence "Attack" 1.0 0.0))

(event Custom|GunCooldown
  (Utilities|Time|SetTimerbyEvent (delegate Custom|Gun%20Recharge) 3.0)
  (Variables|Default|SetOnGunCooldown true))

(event Custom|Gun%20Recharge
  (Variables|Default|SetGunCharge 6)
  (Variables|Default|SetOnGunCooldown false))

(event Input|EnhancedActionEvents|EnhancedInputActionIA_Attack
  (params (ActionValue :type Boolean) (ElapsedSeconds :type Float%20%28double-precision%29) (TriggeredSeconds :type Float%20%28double-precision%29) (InputAction :type Input%20Action%20Object%20Reference :default "/Game/GameContent/Input/Action/IA_Attack.IA_Attack"))
  (:Started
    (switch Utilities|FlowControl|Switch|SwitchonE_State (Variables|Default|GetState)
      (:NewEnumerator1
        (CallFunction|MeleeAttack))
      (:NewEnumerator2
        (CallFunction|RangedAttack)))))

(event Input|EnhancedActionEvents|EnhancedInputActionIA_StateIdle
  (params (ActionValue :type Boolean) (ElapsedSeconds :type Float%20%28double-precision%29) (TriggeredSeconds :type Float%20%28double-precision%29) (InputAction :type Input%20Action%20Object%20Reference :default "/Game/GameContent/Input/Action/IA_StateIdle.IA_StateIdle"))
  (:Started
    (Variables|Default|SetState "NewEnumerator0")
    (Development|PrintString "iDLE")))

(event Input|EnhancedActionEvents|EnhancedInputActionIA_Statemelee
  (params (ActionValue :type Boolean) (ElapsedSeconds :type Float%20%28double-precision%29) (TriggeredSeconds :type Float%20%28double-precision%29) (InputAction :type Input%20Action%20Object%20Reference :default "/Game/GameContent/Input/Action/IA_Statemelee.IA_Statemelee"))
  (:Started
    (Variables|Default|SetState "NewEnumerator1")
    (Development|PrintString "Melee" true true "(R=0.000000,G=1.000000,B=0.043210,A=1.000000)")))

(event Input|EnhancedActionEvents|EnhancedInputActionIA_StateRange
  (params (ActionValue :type Boolean) (ElapsedSeconds :type Float%20%28double-precision%29) (TriggeredSeconds :type Float%20%28double-precision%29) (InputAction :type Input%20Action%20Object%20Reference :default "/Game/GameContent/Input/Action/IA_StateRange.IA_StateRange"))
  (:Started
    (Variables|Default|SetState "NewEnumerator2")
    (Development|PrintString "Rango" true true "(R=1.000000,G=0.122771,B=0.182505,A=1.000000)")))

(event EventBeginPlay
  (CallFunction|ConnectController))

(fn ConstructionScript
  (|CallParentFunction))

(fn RangedAttack
  (if (>= (Variables|Default|GetGunCharge) 0)
    (if (not (Variables|Default|GetOnGunCooldown))
      (CallFunction|GunCooldown)
      (CallFunction|AttackAnim (Variables|/Script/PaperZD.PaperZDAnimationComponent|GetAnimInstance (Variables|Default|GetAnimationComponent)) (Variables|Default|GetRangeSequence)))
    (else
      (Variables|Default|SetGunCharge (- (Variables|Default|GetGunCharge) 1)))))

(fn ConnectController
  (bind _asplayer_controller (Utilities|Casting|CastToPlayerController (Pawn|GetController)))
  (Input|AddMappingContext (PlayerController|LocalPlayerSubsystems|GetEnhancedInputLocalPlayerSubsystem _asplayer_controller) "/Game/GameContent/Input/IMC_Player.IMC_Player" 0 "(bIgnoreAllPressedKeysUntilRelease=True,bForceImmediately=False,bNotifyUserSettings=False)"))

(fn MeleeAttack
  (Default|Spawn (Variables|Componentes|GetBPC_Attack) "/Game/GameContent/Blueprint/Props/Attack/Player/BP_PlayerMelee.BP_PlayerMelee_C" self)
  (CallFunction|AttackAnim (Variables|/Script/PaperZD.PaperZDAnimationComponent|GetAnimInstance (Variables|Default|GetAnimationComponent)) (Variables|Default|GetMeleeSequence)))